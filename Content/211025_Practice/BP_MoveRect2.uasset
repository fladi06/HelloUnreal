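; BP_MoveRect2 is a practice Blueprint that moves a Sphere component around a square path in its relative XY space while IsPlay is true.
; Tick switches on the Movetype state and calls one move function per side, offsetting the sphere by delta time times Speed.
; Each function sets the next direction once the sphere passes FinalPos or zero, looping Right, Top, Left, Bottom without clamping at corners.
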(event `self.ReceiveTick`
  (params (DeltaSeconds :type "Float (single-precision)"))
  (if (`self.isPlay`)
    (switch `/Game/211025_Practice/BP_MoveRect_2` (`self.Movetype`)
      (:`NewEnumerator0`
        (`self.Move Right` DeltaSeconds))
      (:`NewEnumerator1`
        (`self.Move Left` DeltaSeconds))
      (:`NewEnumerator2`
        (`self.Move Top` DeltaSeconds))
      (:`NewEnumerator3`
        (`self.Move Bottom` DeltaSeconds)))))

(fn `Move Bottom`
  (params (Second :type "Float (double-precision)"))
  (bind _sphere (`self.Sphere`))
  (bind (_relativelocation_x _relativelocation_y) (`KismetMathLibrary.BreakVector` (`SceneComponent.RelativeLocation` _sphere)))
  (bind _result (`/Engine/EditorBlueprintResources/StandardMacros.NegateFloat` (* Second (`self.Speed`)))
    (:`  `
      (`SceneComponent.K2_AddRelativeLocation` _sphere (`KismetMathLibrary.MakeVector` 0.0 _result) false false)
      (if (< _relativelocation_y 0.0)
        (set `self.Movetype` "NewEnumerator0")))))

(fn `Move Left`
  (params (Second :type "Float (double-precision)"))
  (bind _sphere (`self.Sphere`))
  (bind _relativelocation_x (`KismetMathLibrary.BreakVector` (`SceneComponent.RelativeLocation` _sphere)))
  (bind _result (`/Engine/EditorBlueprintResources/StandardMacros.NegateFloat` (* Second (`self.Speed`)))
    (:`  `
      (`SceneComponent.K2_AddRelativeLocation` _sphere (`KismetMathLibrary.MakeVector` _result) false false)
      (if (< _relativelocation_x 0.0)
        (set `self.Movetype` "NewEnumerator3")))))

(fn `Move Right`
  (params (Second :type "Float (double-precision)"))
  (bind _sphere (`self.Sphere`))
  (bind _relativelocation_x (`KismetMathLibrary.BreakVector` (`SceneComponent.RelativeLocation` _sphere)))
  (`SceneComponent.K2_AddRelativeLocation` _sphere (`KismetMathLibrary.MakeVector` (* Second (`self.Speed`))) false false)
  (if (> _relativelocation_x (`self.FinalPos`))
    (set `self.Movetype` "NewEnumerator2")))

(fn `Move Top`
  (params (Second :type "Float (double-precision)"))
  (locals (NewLocalVar_0 :type "Vector Structure" :default (0.0 0.0 0.0)))
  (bind _sphere (`self.Sphere`))
  (bind (_relativelocation_x _relativelocation_y) (`KismetMathLibrary.BreakVector` (`SceneComponent.RelativeLocation` _sphere)))
  (`SceneComponent.K2_AddRelativeLocation` _sphere (`KismetMathLibrary.MakeVector` 0.0 (* Second (`self.Speed`))) false false)
  (if (> _relativelocation_y (`self.FinalPos`))
    (set `self.Movetype` "NewEnumerator1")))

(fn `UserConstructionScript`)