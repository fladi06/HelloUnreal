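; BP_ClockBall is an actor that swings back and forth around its roll axis, like a clock pendulum.
; Each Tick plays or reverses a timeline according to IsRight, scaling its value by 45 to set the actor's roll and flipping the flag when it finishes.
; An Addrotation function, not called in these graphs, holds an alternative swing that steps the Center component's roll each call and flips direction beyond ±45 degrees.
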(event `self.ReceiveTick`
  (params (DeltaSeconds :type "Float (single-precision)"))
  (if (`self.IsRight`)
    (bind (_direction _value) (`Timeline|Timeline_0` :!label _label)
      (:`Update`
        (`self.K2_SetActorRotation` (`KismetMathLibrary.MakeRotator` (* _value 45.0))))
      (:`Finished`
        (set `self.IsRight` (not (`self.IsRight`)))))
    (else
      (goto _label :!via `Reverse`))))

(fn `Addrotation`
  (bind _center (`self.Center`))
  (bind _relativerotation_roll (`KismetMathLibrary.BreakRotator` (`SceneComponent.RelativeRotation` _center)))
  (if (`self.IsRight`)
    (`SceneComponent.K2_AddLocalRotation` _center (struct :`Roll` 1.0) false false)
    (if (> _relativerotation_roll 45.0)
      (set `self.IsRight` (not (`self.IsRight`))))
    (else
      (`SceneComponent.K2_AddLocalRotation` _center (struct :`Roll` -1.0) false false)
      (if (< _relativerotation_roll -45.0)
        (set `self.IsRight` (not (`self.IsRight`)))))))

(fn `UserConstructionScript`)