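; BP_Spawn is a practice pawn that flies with camera-relative movement and spawns a BP_MoveRect2 actor at BeginPlay.
; PressP toggles IsPlay on the stored MoveRect reference.
; MoveForward and MoveRight offset the pawn along the camera manager's forward and right vectors without sweep or delta-time scaling.
; Look axes feed controller pitch and yaw, and a test axis prints its value for debugging.
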(event `self.ReceiveBeginPlay`
  (bind _returnvalue (`|SpawnActorFromClass` "/Game/211025_Practice/BP_MoveRect2.BP_MoveRect2_C" (`KismetMathLibrary.MakeTransform` (0.0 0.0 10.0)) "Undefined" "OverrideRootScale" null false null))
  (set `self.MoveRect` _returnvalue))

(event `InputAction|PressP`
  (params (Key :type "Key Structure"))
  (bind _moverect (`self.MoveRect`))
  (:`Pressed`
    (set `/Game/211025_Practice/BP_MoveRect2.isPlay` (not (`/Game/211025_Practice/BP_MoveRect2.isPlay` _moverect)) _moverect)))

(event `InputAxis|Axis Test`
  (params (AxisValue :type "Float (single-precision)"))
  (`KismetSystemLibrary.PrintString` (`KismetStringLibrary.Concat_StrStr` "Axis Test" (`KismetStringLibrary.Conv_DoubleToString` AxisValue))))

(event `InputAxis|MoveForward`
  (params (AxisValue :type "Float (single-precision)"))
  (`self.K2_AddActorWorldOffset` (* (`self.GetActorForwardVector` (`GameplayStatics.GetPlayerCameraManager` 0)) (* AxisValue 10.0))))

(event `InputAxis|MoveRight`
  (params (AxisValue :type "Float (single-precision)"))
  (`self.K2_AddActorWorldOffset` (* (`self.GetActorRightVector` (`GameplayStatics.GetPlayerCameraManager` 0)) (* AxisValue 10.0))))

(event `InputAxis|LookUp`
  (params (AxisValue :type "Float (single-precision)"))
  (`self.AddControllerPitchInput` AxisValue))

(event `InputAxis|LookRIght`
  (params (AxisValue :type "Float (single-precision)"))
  (`self.AddControllerYawInput` AxisValue))

(fn `UserConstructionScript`)