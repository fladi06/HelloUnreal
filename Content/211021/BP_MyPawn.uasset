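; Player pawn for a test scene that spawns four demo motion actors and toggles their playback.
; BeginPlay spawns and stores MoveActor, MoveRect, TimelineActor and RotationBall at fixed heights; PressP flips IsPlay on the first two and calls Toggle on the others.
; Axis inputs fly the pawn along camera forward and right vectors without sweep and drive controller pitch and yaw.
; Enter, HelloWorld and Axis Test inputs only print debug strings.
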(event `self.ReceiveBeginPlay`
  ;[1 1 1] MoveActor Spawn
  (bind _returnvalue (`|SpawnActorFromClass` "/Game/211021/BP_MoveActor.BP_MoveActor_C" (`KismetMathLibrary.MakeTransform` (0.0 0.0 100.0)) "Undefined" "OverrideRootScale" null 0.0 null))
  (set `self.MoveActor` _returnvalue)
  ;[1 1 1] MoveRect Spawn
  (bind _returnvalue_2 (`|SpawnActorFromClass` "/Game/211021/BP_MoveRect.BP_MoveRect_C" (`KismetMathLibrary.MakeTransform` (0.0 0.0 300.0)) "Undefined" "OverrideRootScale" null false null))
  (set `self.MoveRect` _returnvalue_2)
  ;[1 1 1] TimelineActor Spawn
  (bind _returnvalue_3 (`|SpawnActorFromClass` "/Game/211021/BP_TimelineActor.BP_TimelineActor_C" (`KismetMathLibrary.MakeTransform` (0.0 0.0 20.0)) "Undefined" "OverrideRootScale" null null))
  (set `self.TimelineActor` _returnvalue_3)
  ;[1 1 1] RotationBall Spawn
  (bind _returnvalue_4 (`|SpawnActorFromClass` "/Game/211021/BP_RotationBall.BP_RotationBall_C" (`KismetMathLibrary.MakeTransform` (0.0 0.0 1.0)) "Undefined" "OverrideRootScale" null null))
  (set `self.RotationBall` _returnvalue_4))

(event `InputAction|PressP`
  (params (Key :type "Key Structure"))
  (bind _moveactor (`self.MoveActor`))
  ;[1 1 1] PressP -> MoveActor
  (:`Pressed`
    (set `/Game/211021/BP_MoveActor.IsPlay` (not (`/Game/211021/BP_MoveActor.IsPlay` _moveactor)) _moveactor)))

(event `InputAction|PressP`
  (params (Key :type "Key Structure"))
  (bind _moverect (`self.MoveRect`))
  ;[1 1 1] PressP -> MoveRect
  (:`Pressed`
    (set `/Game/211021/BP_MoveRect.IsPlay` (not (`/Game/211021/BP_MoveRect.IsPlay` _moverect)) _moverect)))

(event `InputAction|PressP`
  (params (Key :type "Key Structure"))
  ;[1 1 1] PressP -> Timeline Actor
  (:`Pressed`
    (`/Game/211021/BP_TimelineActor.Toggle` (`self.TimelineActor`))))

(event `InputAction|PressP`
  (params (Key :type "Key Structure"))
  ;[1 1 1] PressP -> Rotation Ball Actor
  (:`Pressed`
    (`/Game/211021/BP_RotationBall.Toggle` (`self.RotationBall`))))

(event `Key|Enter`
  (params (Key :type "Key Structure"))
  (:`Pressed`
    (`KismetSystemLibrary.PrintString` "Enter Pressed" true true (struct :`G` 0.66 :`B` 1.0 :`A` 1.0) 60.0))
  (:`Released`
    (`KismetSystemLibrary.PrintString` "Enter Released" true true (struct :`G` 0.66 :`B` 1.0 :`A` 1.0) 60.0)))

(event `InputAction|HelloWorld`
  (params (Key :type "Key Structure"))
  (:`Pressed`
    (`KismetSystemLibrary.PrintString` "Hello World Pressed" true true (struct :`G` 0.66 :`B` 1.0 :`A` 1.0) 60.0))
  (:`Released`
    (`KismetSystemLibrary.PrintString` "Hello World Released" true true (struct :`G` 0.66 :`B` 1.0 :`A` 1.0) 60.0)))

(event `InputAxis|Axis Test`
  (params (AxisValue :type "Float (single-precision)"))
  (`KismetSystemLibrary.PrintString` (`KismetStringLibrary.Concat_StrStr` "Axis Test" (`KismetStringLibrary.Conv_DoubleToString` AxisValue))))

(event `InputAxis|MoveForward`
  (params (AxisValue :type "Float (single-precision)"))
  (`self.K2_AddActorWorldOffset` (* (`self.GetActorForwardVector` (`GameplayStatics.GetPlayerCameraManager` 0)) (* AxisValue 10.0))))

(event `InputAxis|MoveRight`
  (params (AxisValue :type "Float (single-precision)"))
  (`self.K2_AddActorWorldOffset` (* (`self.GetActorRightVector` (`GameplayStatics.GetPlayerCameraManager` 0)) (* AxisValue 10.0))))

(event `InputAxis|LookUp`
  (params (AxisValue :type "Float (single-precision)"))
  (`self.AddControllerPitchInput` AxisValue))

(event `InputAxis|LookRIght`
  (params (AxisValue :type "Float (single-precision)"))
  (`self.AddControllerYawInput` AxisValue))

(fn `NewFunction_0`)

(fn `UserConstructionScript`)