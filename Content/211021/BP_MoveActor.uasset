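; BP_MoveActor is an actor that slides its Sphere component back and forth along local X while play is toggled on with the P key.
; Tick calls MoveSphere, which moves at constant delta-time-scaled speed and flips IsRight when relative X passes either bound.
; CountTimer, a 100x-rate clock printing zero-padded Korean minutes and seconds only on change, and PrintHello are defined but not called here.
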(event `self.ReceiveTick`
  (params (DeltaSeconds :type "Float (single-precision)"))
  (if (`self.IsPlay`)
    (`self.MoveSphere` DeltaSeconds)))

(event `/Game/211021/BPI_PressP.PressP`
  (set `self.IsPlay` (not (`self.IsPlay`))))

(fn `CountTimer`
  (params (B :type "Float (double-precision)"))
  (bind _output_get (set `self.TotalDist` (+ (* 100.0 B) (`self.TotalDist`))))
  (bind _returnvalue (`KismetStringLibrary.Concat_StrStr` (`self.time` (`KismetMathLibrary.FFloor` (/ _output_get 60.0))) "분" (`self.time` (`KismetMathLibrary.FFloor` (mod _output_get 60.0))) "초"))
  (if (not (`KismetStringLibrary.EqualEqual_StrStr` _returnvalue (`self.Beforestr`)))
    (`KismetSystemLibrary.PrintString` _returnvalue)
    (set `self.Beforestr` _returnvalue)))

(fn `MoveSphere`
  (params (A :type "Float (double-precision)"))
  (bind _returnvalue (* A 300.0))
  (bind _sphere (`self.Sphere`))
  (bind _relativelocation_x (`KismetMathLibrary.BreakVector` (`SceneComponent.RelativeLocation` (`self.Sphere`))))
  (bind _relativelocation_x_2 (`KismetMathLibrary.BreakVector` (`SceneComponent.RelativeLocation` (`self.Sphere`))))
  (if (`self.is Right`)
    (`SceneComponent.K2_AddLocalOffset` _sphere (`KismetMathLibrary.MakeVector` _returnvalue) false false)
    (if (> _relativelocation_x_2 200.0)
      (set `self.is Right` false))
    (else
      (bind _result (`/Engine/EditorBlueprintResources/StandardMacros.NegateFloat` _returnvalue)
        (:`  `
          (`SceneComponent.K2_AddLocalOffset` _sphere (`KismetMathLibrary.MakeVector` _result) false false)
          (if (< _relativelocation_x 0.0)
            (set `self.is Right` true)))))))

(fn `PrintHello`
  (`KismetSystemLibrary.PrintString` "Hello, BP_MoveActor"))

(fn `time`
  (params (NewParam :type Integer))
  (returns (str00 :type String))
  (if (< NewParam 10)
    (return (`KismetStringLibrary.Concat_StrStr` "0" (`KismetStringLibrary.Conv_IntToString` NewParam)))
    (else
      (return (`KismetStringLibrary.Conv_IntToString` NewParam)))))

(fn `UserConstructionScript`)