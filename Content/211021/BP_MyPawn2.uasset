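; BP_MyPawn2 is a pawn that broadcasts a P key press to other actors through the BPI_PressP interface.
; On BeginPlay it scans all actors in the world and caches those implementing the interface in an array.
; Pressing P loops over that array, rechecks the interface and calls PressPMessage on each, so no casts to specific classes are needed.
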(event `self.ReceiveBeginPlay`
  (bind _outactors (`GameplayStatics.GetAllActorsOfClass` "/Script/Engine.Actor"))
  (for _array_element _outactors
    (if (`KismetSystemLibrary.DoesImplementInterface` _array_element "/Game/211021/BPI_PressP.BPI_PressP_C")
      (`KismetArrayLibrary.Array_Add` (`self.Actor`) _array_element))))

(event `Key|P`
  (params (Key :type "Key Structure"))
  (:`Pressed`
    (for _array_element (`self.Actor`)
      (if (`KismetSystemLibrary.DoesImplementInterface` _array_element "/Game/211021/BPI_PressP.BPI_PressP_C")
        (message `/Game/211021/BPI_PressP.PressP` _array_element)))))

(fn `NewFunction_0`)

(fn `UserConstructionScript`)