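; BP_RotationBall is an actor that swings its Center component back and forth in roll like a pendulum, toggled by the PressP event.
; PlayEvent runs a timeline scaled by 45 degrees, flipping IsRight on finish to alternate Play and Reverse; StopEvent halts it.
; ClockRotation is an uncalled, step-based alternative that nudges roll each call and flips direction beyond the 45-degree limits.
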(event `/Game/211021/BPI_PressP.PressP`
  (if (`self.IsPlay`)
    (`self.StopEvent`)
    (else
      (`self.PlayEvent`))))

(event `PlayEvent`
  (set `self.IsPlay` true)
  (if (`self.IsRight`) :!label _label
    (bind (_direction _value) (`Timeline|Timeline_0` :!label _label_2)
      (:`Update`
        (`SceneComponent.K2_SetRelativeRotation` (`self.Center`) (`KismetMathLibrary.MakeRotator` (* _value 45.0)) false false))
      (:`Finished`
        (set `self.IsRight` (not (`self.IsRight`)))
        (goto _label)))
    (else
      (goto _label_2 :!via `Reverse`))))

(event `StopEvent`
  (set `self.IsPlay` false)
  (goto _label_2 :!via `Stop`))

(fn `ClockRotation`
  (bind _center (`self.Center`))
  (bind _relativerotation_roll (`KismetMathLibrary.BreakRotator` (`SceneComponent.RelativeRotation` _center)))
  (if (`self.IsRight`)
    (`SceneComponent.K2_AddLocalRotation` _center (struct :`Roll` 1.0) false false)
    (if (> _relativerotation_roll 45.0)
      (set `self.IsRight` (not (`self.IsRight`))))
    (else
      (`SceneComponent.K2_AddLocalRotation` _center (struct :`Roll` -1.0) false false)
      (if (< _relativerotation_roll -45.0)
        (set `self.IsRight` (not (`self.IsRight`)))))))

(fn `UserConstructionScript`)