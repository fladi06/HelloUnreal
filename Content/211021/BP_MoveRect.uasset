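; BP_MoveRect is a Blueprint that moves its Sphere component around a square path in relative XY space, with P toggling movement on and off.
; While playing, Tick switches on the Movetype state and calls one of four directional functions, each stepping the sphere by Speed scaled by delta time.
; Each function sets the next direction once the sphere passes zero or Destpos, cycling Right, Top, Left, Bottom.
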(event `self.ReceiveTick`
  (params (DeltaSeconds :type "Float (single-precision)"))
  (if (`self.IsPlay`)
    (switch `/Game/211021/Enum_Move` (`self.Movetype`)
      (:`NewEnumerator0`
        (`self.MoveRight` DeltaSeconds))
      (:`NewEnumerator1`
        (`self.MoveLeft` DeltaSeconds))
      (:`NewEnumerator2`
        (`self.MoveTop` DeltaSeconds))
      (:`NewEnumerator3`
        (`self.MoveBottom` DeltaSeconds)))))

(event `/Game/211021/BPI_PressP.PressP`
  (set `self.IsPlay` (not (`self.IsPlay`))))

(fn `MoveBottom`
  (params (DeltaSecond :type "Float (double-precision)"))
  (bind (_relativelocation_x _relativelocation_y) (`KismetMathLibrary.BreakVector` (`SceneComponent.RelativeLocation` (`self.Sphere`))))
  (bind _result (`/Engine/EditorBlueprintResources/StandardMacros.NegateFloat` (* DeltaSecond (`self.speed`)))
    (:`  `
      (`SceneComponent.K2_AddRelativeLocation` (`self.Sphere`) (`KismetMathLibrary.MakeVector` 0.0 _result) false false)
      (if (< _relativelocation_y 0.0)
        (set `self.Movetype` "NewEnumerator0")))))

(fn `MoveLeft`
  (params (DeltaSecond :type "Float (double-precision)"))
  (bind _sphere (`self.Sphere`))
  (bind _relativelocation_x (`KismetMathLibrary.BreakVector` (`SceneComponent.RelativeLocation` _sphere)))
  (bind _result (`/Engine/EditorBlueprintResources/StandardMacros.NegateFloat` (* DeltaSecond (`self.speed`)))
    (:`  `
      (`SceneComponent.K2_AddRelativeLocation` _sphere (`KismetMathLibrary.MakeVector` _result) false false)
      (if (< _relativelocation_x 0.0)
        (set `self.Movetype` "NewEnumerator3")))))

(fn `MoveRight`
  (params (DeltaSecond :type "Float (double-precision)"))
  (bind _sphere (`self.Sphere`))
  (bind _relativelocation_x (`KismetMathLibrary.BreakVector` (`SceneComponent.RelativeLocation` _sphere)))
  (`SceneComponent.K2_AddRelativeLocation` _sphere (`KismetMathLibrary.MakeVector` (* DeltaSecond (`self.speed`))) false false)
  (if (> _relativelocation_x (`self.Destpos`))
    (set `self.Movetype` "NewEnumerator2")))

(fn `MoveTop`
  (params (DeltaSecond :type "Float (double-precision)"))
  (bind _sphere (`self.Sphere`))
  (bind (_relativelocation_x _relativelocation_y) (`KismetMathLibrary.BreakVector` (`SceneComponent.RelativeLocation` _sphere)))
  (`SceneComponent.K2_AddRelativeLocation` _sphere (`KismetMathLibrary.MakeVector` 0.0 (* DeltaSecond (`self.speed`))) false false)
  (if (> _relativelocation_y (`self.Destpos`))
    (set `self.Movetype` "NewEnumerator1")))

(fn `UserConstructionScript`)